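; BP_Enemy is an enemy character Blueprint that runs the BT_Enemy behavior tree and mirrors its behavior enum to the blackboard.
; Seeing a pawn refreshes and shows the health widget; if it is the player, the behavior state switches unless a specific state blocks it.
; Damage reduces health, with zero health from StatsComp triggering death handling.
; Events also toggle the lock-on widget and play random attack montages, storing their duration.
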(event `self.ReceiveBeginPlay`
  (`AIController.RunBehaviorTree` (`AIBlueprintHelperLibrary.GetAIController` self) "/Game/Characters/Enemy/AI/BT_Enemy.BT_Enemy")
  (`BlackboardComponent.SetValueAsEnum` (`AIBlueprintHelperLibrary.GetBlackboard` null) "ebehavior" (`self.ebehavior`)))

(event `self.ReceiveAnyDamage`
  (params (Damage :type "Float (single-precision)") (DamageType :type "DamageType Object Reference") (InstigatedBy :type "Controller Object Reference") (DamageCauser :type "Actor Object Reference"))
  (`self.ReduceHealth` Damage))

(event `self.ShowLockOnUI`
  (`SceneComponent.SetVisibility` (`self.LockOnWidget`) true false))

(event `self.HideLockOnUI`
  (`SceneComponent.SetVisibility` (`self.LockOnWidget`) false false))

(event `Attack`
  (bind _returnvalue (`self.PlayAnimMontage` (`KismetArrayLibrary.Array_Random` (`self.AttackAnims`))))
  (set `self.AttackDuration` _returnvalue))

(event `self.PawnSensing.OnSeePawn`
  (params (Pawn :type "Pawn Object Reference"))
  (bind _aswbp_enemy (cast `/Game/UI/WBP_Enemy` (`WidgetComponent.GetWidget` (`self.HealthWidget`))))
  (`/Game/UI/WBP_Enemy.SetHealth` _aswbp_enemy (`self.GetPercentage` "Health" "MaxHealth"))
  (`SceneComponent.SetVisibility` (`self.HealthWidget`) true false)
  (if (and (== Pawn (`GameplayStatics.GetPlayerCharacter` 0)) (`|EnumInequality` (`self.ebehavior`) "NewEnumerator0"))
    (set `self.ebehavior` "NewEnumerator3")
    (`BlackboardComponent.SetValueAsEnum` (`AIBlueprintHelperLibrary.GetBlackboard` null) "ebehavior" (`self.ebehavior`))))

(event `self.StatsComp.OnZeroHealthDelegate`
  (params (IsZero :type Boolean))
  (`self.HandleDeath`))

(fn `UserConstructionScript`)