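; Boss character that runs the BT_Boss behavior tree and shows its own health bar to the player.
; Pawn sensing detects the player and, on the first sighting, creates the WBP_Boss widget.
; Damage reduces health, while stats component delegates update the bar and, at zero health, trigger death handling and remove it.
; Lock-on events toggle a marker widget, and health-change callbacks only print values.
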(event `self.ReceiveBeginPlay`
  (`AIController.RunBehaviorTree` (`AIBlueprintHelperLibrary.GetAIController` self) "/Game/Characters/Boss/AI/BT_Boss.BT_Boss")
  (add `EnemyCharacter.OnMaxHealthChanged` (delegate `OnMaxHealthChanged_Event`))
  (add `EnemyCharacter.OnHealthChanged` (delegate `OnHealthChanged_Event`)))

(event `self.ReceiveTick`
  (params (DeltaSeconds :type "Float (single-precision)")))

(event `OnMaxHealthChanged_Event`
  (params (newValue :type "Float (single-precision)"))
  (`KismetSystemLibrary.PrintString` (`KismetStringLibrary.Conv_DoubleToString` newValue)))

(event `OnHealthChanged_Event`
  (params (newValue :type "Float (single-precision)"))
  (`KismetSystemLibrary.PrintString` (`KismetStringLibrary.Conv_DoubleToString` newValue)))

(event `ShowLockOnUI_1`
  (`SceneComponent.SetVisibility` (`self.LockOnWidget`) true false))

(event `HideLockOnUI_1`
  (`SceneComponent.SetVisibility` (`self.LockOnWidget`) false false))

(event `self.StatsComp.OnUpdateHealthUIDelegate`
  (params (Percentage :type "Float (single-precision)"))
  (`/Game/UI/WBP_Boss.Set Health` (`self.Boss Widget`) Percentage))

(event `self.ReceiveAnyDamage`
  (params (Damage :type "Float (single-precision)") (DamageType :type "DamageType Object Reference") (InstigatedBy :type "Controller Object Reference") (DamageCauser :type "Actor Object Reference"))
  (`self.ReduceHealth` Damage))

(event `self.PawnSensing.OnSeePawn`
  (params (Pawn :type "Pawn Object Reference"))
  (`self.DetectPawn` Pawn (`GameplayStatics.GetPlayerPawn` 0))
  (`/Engine/EditorBlueprintResources/StandardMacros.DoOnce` false
    (:`Completed`
      (bind _returnvalue (`|CreateWidget` "/Game/UI/WBP_Boss.WBP_Boss_C"))
      (bind _output_get (set `self.Boss Widget` _returnvalue))
      (`UserWidget.AddToViewport` _output_get 0)
      (`/Game/UI/WBP_Boss.Set Health` (`self.Boss Widget`) (`self.GetPercentage` "Health" "MaxHealth")))))

(event `self.StatsComp.OnZeroHealthDelegate`
  (params (IsZero :type Boolean))
  (`self.HandleDeath`)
  (`Widget.RemoveFromParent` (`self.Boss Widget`)))

(fn `UserConstructionScript`)