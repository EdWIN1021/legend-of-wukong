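; GA_Attack is a Gameplay Ability that plays a chained combo attack, one montage per activation.
; On activation it clears any pending reset timer and plays the montage mapped to ComboCount, then increments the count or wraps to 1 after the last.
; When the montage completes, blends out, is interrupted or cancelled, the ability ends and starts a short timer that resets the combo unless another attack clears it.
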(event `self.K2_ActivateAbility`
  (`KismetSystemLibrary.K2_ClearAndInvalidateTimerHandle` (`self.TimberHandler`))
  (`KismetSystemLibrary.PrintString` (`KismetStringLibrary.Conv_IntToString` (`self.ComboCount`)))
  (`AbilityTask_PlayMontageAndWait.CreatePlayMontageAndWaitProxy` "None" (`BlueprintMapLibrary.Map_Find` (`self.AttackMontages`) (`self.ComboCount`))
    (:`then`
      (if (== (`self.ComboCount`) (`BlueprintMapLibrary.Map_Length` (`self.AttackMontages`)))
        (`self.RestComboCount`)
        (else
          (`/Engine/EditorBlueprintResources/StandardMacros.IncrementInt` (`self.ComboCount`)))))
    (:`OnCompleted`
      (`self.K2_EndAbility` :!label _label)
      (bind _returnvalue (`KismetSystemLibrary.K2_SetTimerDelegate` (delegate `RestComboCount`) 0.3))
      (set `self.TimberHandler` _returnvalue))
    (:`OnBlendOut`
      (goto _label))
    (:`OnInterrupted`
      (goto _label))
    (:`OnCancelled`
      (goto _label))))

(event `RestComboCount`
  (set `self.ComboCount` 1))