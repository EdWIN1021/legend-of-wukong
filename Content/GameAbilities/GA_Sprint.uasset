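; Gameplay Ability that makes the Wukong player character sprint by raising its max walk speed.
; On activation it binds to the player controller's finish-sprint event, boosts the CharacterMovement speed and commits the ability cost.
; The finish-sprint event ends the ability, which restores normal walk speed and tells the controller to re-enable stamina restoration.
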(event `self.K2_ActivateAbility`
  (bind _asbp_wukong_player_controller (cast `/Game/PlayerController/BP_WukongPlayerController` (`GameplayStatics.GetPlayerController` 0)))
  (add `WukongPlayerController.OnFinishSprint` _asbp_wukong_player_controller (delegate `OnFinishSprint_Event_0`))
  (bind _asbp_wukong (cast `/Game/Characters/Wukong/Blueprints/BP_Wukong` (`self.GetAvatarActorFromActorInfo`)))
  (bind _output_get (set `self.As BP Wukong` _asbp_wukong))
  (set `CharacterMovementComponent.MaxWalkSpeed` 1000.0 (`Character.CharacterMovement` _output_get))
  (`self.K2_CommitAbilityCost` false))

(event `OnFinishSprint_Event_0`
  (`self.K2_EndAbility`))

(event `self.K2_OnEndAbility`
  (params (bWasCancelled :type Boolean))
  (set `CharacterMovementComponent.MaxWalkSpeed` 500.0 (`Character.CharacterMovement` (`self.As BP Wukong`)))
  (bind _asbp_wukong_player_controller (cast `/Game/PlayerController/BP_WukongPlayerController` (`GameplayStatics.GetPlayerController` 0)))
  (`WukongPlayerController.EnableRestoreStamina` _asbp_wukong_player_controller))